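; Presentation camera actor that spawns its own CameraActor, becomes the player's view target when active, and can chain to a linked next camera.
; After eight seconds it blends to NextCamera unless the Controller reports it is controlled.
; Tick optionally rotates the view, adjusting the step at rotation limits.
; ShowMesh advances an index to toggle Linda's visibility, then show and hide cutscene and outro videos in UIPanel widgets; Playsound plays only while active.
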(event `onActive`
  (`KismetSystemLibrary.Delay` 8.0)
  (bind _outactors (`GameplayStatics.GetAllActorsOfClass` "/Game/Blueprints/Controller.Controller_C"))
  (bind _newparam (`/Game/Blueprints/Controller.isControlled` (`|GetArrayItem` _outactors)))
  (if (not _newparam)
    (`self.nextCam`)))

(event `self.ReceiveTick`
  (params (DeltaSeconds :type "Float (single-precision)"))
  (bind _rotation (`self.Rotation`))
  (bind _returnvalue (`KismetMathLibrary.Conv_VectorToRotator` (+ (`KismetMathLibrary.Conv_RotatorToVector` (`self.K2_GetActorRotation`)) (`KismetMathLibrary.MakeVector` 0.0 (`self.Rotation/tick`)))))
  (if (and (`self.active`) (`self.rot`))
    (set `self.Rotation` (+ (`self.Rotation`) (`self.Rotation/tick`)))
    (`self.K2_SetActorRotation` (`self.Camera`) _returnvalue true)
    (`self.K2_SetActorRotation` _returnvalue true)
    (if (or (>= _rotation 1.0) (<= _rotation -1.0))
      (`/Engine/EditorBlueprintResources/StandardMacros.DoOnce` false :!label _label
        (:`Completed`
          (`/Engine/EditorBlueprintResources/StandardMacros.NegateFloat` (`self.Rotation/tick`))))
      (else
        (goto _label :!via `Reset`)))))

(event `self.ReceiveBeginPlay`
  (bind _returnvalue (`|SpawnActorFromClass` "/Script/Engine.CameraActor" (`self.GetTransform`) "AlwaysSpawn" "OverrideRootScale"))
  (set `self.Camera` _returnvalue)
  (`self.SetActive` (`self.active`)))

(fn `isActive`
  (returns (active :type Boolean))
  (return (`self.active`)))

(fn `nextCam`
  (returns (NewParam :type Boolean))
  (if (`self.active`)
    (set `self.was_active` true)
    (`self.SetActive` false)
    (`self.SetActive` (`self.Next Camera`) true 2.0)
    (else
      (set `self.was_active` false)))
  (return (`self.was_active`)))

(fn `Playsound`
  (params (Sound :type "SoundBase Object Reference"))
  (bind _audio (`self.Audio`))
  (bind _active (`self.isActive`))
  (if _active
    (set `AudioComponent.Sound` Sound _audio)
    (`AudioComponent.Play` _audio 0.0)))

(fn `SetActive`
  (params (active :type Boolean) (`blend time` :type "Float (double-precision)"))
  (if active
    (`self.onActive`)
    (`PlayerController.SetViewTargetWithBlend` (`GameplayStatics.GetPlayerController` 0) (`self.Camera`) `blend time` "VTBlend_Linear" 0.0 false))
  (set `self.active` active))

(fn `showMesh`
  (params (show :type Boolean))
  (bind _media (`self.Media`))
  (bind _media_2 (`self.Media`))
  (bind _output_get (set `self.Index` (+ (`self.Index`) 1)))
  (switch `int` _output_get
    (:`0`
      (`SceneComponent.SetVisibility` (`self.linda`) show true :!label _label))
    (:`1`
      (goto _label))
    (:`2`
      (`MediaPlayer.OpenSource` _media "/Game/Movies/CutScene.CutScene")
      (bind _foundwidgets (`WidgetBlueprintLibrary.GetAllWidgetsOfClass` "/Game/Assets/Blueprints/UIPanel.UIPanel_C"))
      (for _array_element _foundwidgets
        (`Widget.SetVisibility` (`/Game/Assets/Blueprints/UIPanel.Image_331` _array_element) "Visible")
        (`MediaPlayer.Play` _media)))
    (:`3`
      (bind _foundwidgets_2 (`WidgetBlueprintLibrary.GetAllWidgetsOfClass` "/Game/Assets/Blueprints/UIPanel.UIPanel_C"))
      (for _array_element_2 _foundwidgets_2
        (`Widget.SetVisibility` (`/Game/Assets/Blueprints/UIPanel.Image_331` _array_element_2) "Collapsed")))
    (:`4`
      (`MediaPlayer.OpenSource` _media_2 "/Game/Movies/Outro.Outro")
      (bind _foundwidgets_3 (`WidgetBlueprintLibrary.GetAllWidgetsOfClass` "/Game/Assets/Blueprints/UIPanel.UIPanel_C"))
      (for _array_element_3 _foundwidgets_3
        (`Widget.SetVisibility` (`/Game/Assets/Blueprints/UIPanel.Image_331` _array_element_3) "Visible")
        (`MediaPlayer.Play` _media_2)))
    (:`5`
      (bind _foundwidgets_4 (`WidgetBlueprintLibrary.GetAllWidgetsOfClass` "/Game/Assets/Blueprints/UIPanel.UIPanel_C"))
      (for _array_element_4 _foundwidgets_4
        (`Widget.SetVisibility` (`/Game/Assets/Blueprints/UIPanel.Image_331` _array_element_4) "Collapsed")))))

(fn `toggleRotation`
  (set `self.rot` (not (`self.rot`))))

(fn `UserConstructionScript`)